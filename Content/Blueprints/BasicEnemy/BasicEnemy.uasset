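; BasicEnemy is an AI enemy character that detects the player and can be marked by target lock-on.
; AI perception and an attack range overlap write PlayerInSight and InRange flags to its Blackboard.
; TargetLockon flip-flops a cone marker's visibility and the mesh's custom depth, while a timeline started on BeginPlay animates the cone's offset.
; A helper function sets the max walk speed.
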(event `self.AIPerception.OnTargetPerceptionUpdated`
  (params (Actor :type "Actor Object Reference") (Stimulus :type "AIStimulus Structure"))
  (bind _playerinsight (`self.PlayerInSight`))
  (bind _returnvalue (`AIBlueprintHelperLibrary.GetBlackboard` self))
  ;[1 1 1] Detect Player
  (if (and (`self.ActorHasTag` Actor "Player") (`.bSuccessfullySensed` (break `AIStimulus` Stimulus)))
    (`BlackboardComponent.SetValueAsBool` _returnvalue _playerinsight true)
    (else
      (`BlackboardComponent.SetValueAsBool` _returnvalue _playerinsight false))))

(event `self.AttackRange.OnComponentBeginOverlap`
  (params (OverlappedComponent :type "PrimitiveComponent Object Reference") (OtherActor :type "Actor Object Reference") (OtherComp :type "PrimitiveComponent Object Reference") (OtherBodyIndex :type Integer) (bFromSweep :type Boolean) (SweepResult :type "HitResult Structure (by ref)"))
  ;[1 1 1] See if player is in attack range
  (cast `/Game/Blueprints/ThirdPersonCharacter` OtherActor)
  (`BlackboardComponent.SetValueAsBool` (`AIBlueprintHelperLibrary.GetBlackboard` (`AIBlueprintHelperLibrary.GetAIController` self)) (`self.InRange`) true))

(event `self.AttackRange.OnComponentEndOverlap`
  (params (OverlappedComponent :type "PrimitiveComponent Object Reference") (OtherActor :type "Actor Object Reference") (OtherComp :type "PrimitiveComponent Object Reference") (OtherBodyIndex :type Integer))
  ;[1 1 1] See if player is in attack range
  (cast `/Game/Blueprints/ThirdPersonCharacter` OtherActor)
  (`BlackboardComponent.SetValueAsBool` (`AIBlueprintHelperLibrary.GetBlackboard` (`AIBlueprintHelperLibrary.GetAIController` self)) (`self.InRange`) false))

(event `self.ReceiveBeginPlay`
  (bind (_direction _animpath) (`Timeline|TargetAnim` :!via `PlayFromStart`)
    (:`Update`
      (`SceneComponent.K2_AddLocalOffset` (`self.Cone`) _animpath false false))))

(event `/Game/Blueprints/LockOnBPI.TargetLockOn`
  (bind _cone (`self.Cone`))
  (bind _mesh (`self.Mesh`))
  (`/Engine/EditorBlueprintResources/StandardMacros.FlipFlop`
    (:`A`
      (`SceneComponent.SetVisibility` _cone true false)
      (`PrimitiveComponent.SetRenderCustomDepth` _mesh true))
    (:`B`
      (`SceneComponent.SetVisibility` _cone false false)
      (`PrimitiveComponent.SetRenderCustomDepth` _mesh false))))

(fn `Update Walk Speed`
  (params (`New Walk Speed` :type "Float (double-precision)"))
  (set `CharacterMovementComponent.MaxWalkSpeed` `New Walk Speed` (`self.CharacterMovement`)))

(fn `UserConstructionScript`)