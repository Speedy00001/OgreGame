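; Behavior tree task that makes a BasicEnemy chase the player character.
; On execute it adds an "Attacking" tag to the pawn, shows the enemy's health bar and switches its walk speed to the chase speed.
; It then runs AI MoveTo targeting the player within an acceptance radius, finishing with success on arrival and failure if the move or the BasicEnemy cast fails.
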(event `self.ReceiveExecuteAI`
  (params (OwnerController :type "AIController Object Reference") (ControlledPawn :type "Pawn Object Reference"))
  (bind _returnvalue (`GameplayStatics.GetPlayerCharacter` 0))
  (`KismetArrayLibrary.Array_Add` (`Actor.Tags` ControlledPawn) "Attacking")
  (bind _asbasic_enemy (cast `/Game/Blueprints/BasicEnemy/BasicEnemy` ControlledPawn)
    (:`then`
      (`SceneComponent.SetVisibility` (`/Game/Blueprints/BasicEnemy/BasicEnemy.HealthBar` _asbasic_enemy) true false)
      (`/Game/Blueprints/BasicEnemy/BasicEnemy.Update Walk Speed` _asbasic_enemy (`self.ChaseSpeed`))
      (`|AIMoveTo` ControlledPawn (`Actor.K2_GetActorLocation` _returnvalue) _returnvalue (`self.Radius`)
        (:`OnSuccess`
          (`self.FinishExecute` true))
        (:`OnFail`
          (`self.FinishExecute` false :!label _label))))
    (:`CastFailed`
      (goto _label))))