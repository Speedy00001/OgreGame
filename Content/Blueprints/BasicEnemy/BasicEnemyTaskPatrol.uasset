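; Behavior Tree task that sends a BasicEnemy patrolling to a random reachable navmesh point around its current location.
; On execute it hides the enemy's health bar, sets patrol walk speed, then uses AI MoveTo toward a point within the patrol radius.
; It finishes successfully whether the move succeeds or fails, but never calls Finish Execute if the cast or point search fails.
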(event `self.ReceiveExecuteAI`
  (params (OwnerController :type "AIController Object Reference") (ControlledPawn :type "Pawn Object Reference"))
  (bind (_randomlocation _returnvalue) (`NavigationSystemV1.K2_GetRandomReachablePointInRadius` (`Actor.K2_GetActorLocation` ControlledPawn) (`self.PatrolRadius`) null "/Script/AIModule.NavFilter_AIControllerDefault"))
  (bind _asbasic_enemy (cast `/Game/Blueprints/BasicEnemy/BasicEnemy` ControlledPawn))
  (`SceneComponent.SetVisibility` (`/Game/Blueprints/BasicEnemy/BasicEnemy.HealthBar` _asbasic_enemy) false false)
  (`/Game/Blueprints/BasicEnemy/BasicEnemy.Update Walk Speed` _asbasic_enemy (`self.PatrolSpeed`))
  (if _returnvalue
    (`|AIMoveTo` ControlledPawn _randomlocation null
      (:`OnSuccess`
        (`self.FinishExecute` true))
      (:`OnFail`
        (`self.FinishExecute` true)))))