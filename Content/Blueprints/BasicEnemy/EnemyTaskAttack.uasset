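; Behavior tree task that makes a BasicEnemy play its attack animation.
; Each AI tick checks the pawn's current montage, resetting a DoOnce during flinch or attack montages and entering it otherwise.
; When the DoOnce fires, it zeroes walk speed and plays the attack montage, re-arming shortly after completion or interruption.
; The task never calls Finish Execute or restores walk speed itself.
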(event `self.ReceiveTickAI`
  (params (OwnerController :type "AIController Object Reference") (ControlledPawn :type "Pawn Object Reference") (DeltaSeconds :type "Float (single-precision)"))
  (bind _asbasic_enemy (cast `/Game/Blueprints/BasicEnemy/BasicEnemy` ControlledPawn))
  (bind _returnvalue (`Character.GetCurrentMontage` _asbasic_enemy))
  (if (or (== _returnvalue "/Game/Characters/NPC/Ninja/Animations/FlinchMontage.FlinchMontage") (== _returnvalue "/Game/Characters/NPC/Ninja/Animations/Attack_Montage.Attack_Montage"))
    (goto _label :!via `Reset`)
    (else
      (`/Engine/EditorBlueprintResources/StandardMacros.DoOnce` false :!label _label
        (:`Completed`
          (set `CharacterMovementComponent.MaxWalkSpeed` 0.0 (`Character.CharacterMovement` _asbasic_enemy))
          (`|PlayMontage` (`Character.Mesh` _asbasic_enemy) (`self.AttackAnim`)
            (:`OnCompleted`
              _)
            (:`OnInterrupted`
              _))
          (`KismetSystemLibrary.Delay` 0.2)
          (goto _label :!via `Reset`))))))