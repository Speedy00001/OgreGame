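; Checkpoint trigger actor that saves the player's location the first time anything overlaps its Box.
; It reads the ThirdPersonCharacter's position and shows an animated Checkpoint widget, later reversing the animation and removing it.
; The location is written to a Save_Blueprint, loaded from SaveSlot or newly created.
; New saves go to SaveSlot, but updated existing saves are written with an empty slot name.
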(event `self.Box.OnComponentBeginOverlap`
  (params (OverlappedComponent :type "PrimitiveComponent Object Reference") (OtherActor :type "Actor Object Reference") (OtherComp :type "PrimitiveComponent Object Reference") (OtherBodyIndex :type Integer) (bFromSweep :type Boolean) (SweepResult :type "HitResult Structure (by ref)"))
  (bind _save_slot (`self.Save_Slot`))
  (bind _player_location (`self.Player_Location`))
  (`/Engine/EditorBlueprintResources/StandardMacros.DoOnce` false
    (:`Completed`
      (`|ExecutionSequence`
        (:`then_0`
          (bind _asthird_person_character (cast `/Game/Blueprints/ThirdPersonCharacter` (`GameplayStatics.GetPlayerCharacter` 0)))
          (set `self.Player_Location` (`self.K2_GetActorLocation` _asthird_person_character))
          (bind _returnvalue (`|CreateWidget` "/Game/UI/Checkpoint.Checkpoint_C"))
          (`UserWidget.AddToViewport` _returnvalue 0)
          (`UserWidget.PlayAnimation` _returnvalue (`/Game/UI/Checkpoint.Checkpoint_Animation` _returnvalue) 0.0 1 "Forward" 1.0))
        (:`then_1`
          (bind _returnvalue_2 (`GameplayStatics.DoesSaveGameExist` _save_slot))
          (if _returnvalue_2
            (bind _returnvalue_3 (`GameplayStatics.LoadGameFromSlot` _save_slot))
            (bind _assave_blueprint (cast `/Game/Blueprints/Save_BP/Save_Blueprint` _returnvalue_3))
            (set `/Game/Blueprints/Save_BP/Save_Blueprint.Player_Location_Save` _player_location _assave_blueprint)
            (`GameplayStatics.SaveGameToSlot` _assave_blueprint)
            (`KismetSystemLibrary.Delay` 2.0)
            (bind _checkpoint_animation (`/Game/UI/Checkpoint.Checkpoint_Animation` _returnvalue))
            (`UserWidget.PlayAnimation` _returnvalue _checkpoint_animation 0.0 1 "Reverse" 1.0)
            (`KismetSystemLibrary.Delay` 0.5)
            (`Widget.RemoveFromParent` _returnvalue)
            (else
              (bind _returnvalue_4 (`GameplayStatics.CreateSaveGameObject` "/Game/Blueprints/Save_BP/Save_Blueprint.Save_Blueprint_C"))
              (set `/Game/Blueprints/Save_BP/Save_Blueprint.Player_Location_Save` _player_location _returnvalue_4)
              (`GameplayStatics.SaveGameToSlot` _returnvalue_4 (`self.Save_Slot`))
              (`KismetSystemLibrary.Delay` 2.0)
              (`UserWidget.PlayAnimation` _returnvalue _checkpoint_animation 0.0 1 "Reverse" 1.0)
              (`KismetSystemLibrary.Delay` 0.5)
              (`Widget.RemoveFromParent` _returnvalue))))))))

(fn `UserConstructionScript`)